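; BP_Cube is an interactable box object that so far only prints a debug message when used.
; Its Interact event runs when either CanPressE or EnemyCanOpen is set, with CanInteract as a re-entry lock.
; If not Engaged, it prints and unlocks after a short delay.
; If Engaged, it clears that flag and leaves the lock closed.
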(event `/Game/Blueprints/Objects/BPI_Interact.Interact`
  ; c
  (if (or (`self.CanPressE`) (`self.EnemyCanOpen`))
    (if (`self.CanInteract`)
      (set `self.CanInteract` false)
      (if (`self.Engaged`)
        (set `self.Engaged` false)
        (else
          (set `self.Engaged` false)
          (`KismetSystemLibrary.PrintString` "Box interacted")
          (`KismetSystemLibrary.Delay` 0.2)
          (set `self.CanInteract` true))))))

(fn `UserConstructionScript`
  (`parent.UserConstructionScript`))