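; BP_PlayerAthlete is a player character Blueprint that adds sprinting, crouching and sliding through Enhanced Input.
; Holding sprint raises walk speed, while crouch on the ground toggles crouch, or starts a slide when sprinting.
; The slide crouches the character and uses a timeline to lerp crouched speed from fast to slow, then uncrouches, with a flag blocking re-entry.
; Attack input only prints a debug string.
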(event `EnhancedInput|/Game/Input/Actions/IA_Crouch`
  (params (ActionValue :type Boolean) (ElapsedSeconds :type "Float (double-precision)") (TriggeredSeconds :type "Float (double-precision)") (InputAction :type "InputAction Object Reference" :default "/Game/Input/Actions/IA_Crouch.IA_Crouch"))
  (:`Triggered`
    (`KismetSystemLibrary.PrintString` "CROUCH")))

(event `EnhancedInput|/Game/Input/Actions/IA_Sprint`
  (params (ActionValue :type Boolean) (ElapsedSeconds :type "Float (double-precision)") (TriggeredSeconds :type "Float (double-precision)") (InputAction :type "InputAction Object Reference" :default "/Game/Input/Actions/IA_Sprint.IA_Sprint"))
  (bind _charactermovement (`self.CharacterMovement`))
  ; Sprint
  (:`Triggered`
    (set `CharacterMovementComponent.MaxWalkSpeed` 600.0 _charactermovement)
    (set `self.Sprinting` true))
  (:`Completed`
    (set `CharacterMovementComponent.MaxWalkSpeed` 300.0 _charactermovement)
    (set `self.Sprinting` false)))

(event `EnhancedInput|/Game/Input/Actions/IA_Crouch`
  (params (ActionValue :type Boolean) (ElapsedSeconds :type "Float (double-precision)") (TriggeredSeconds :type "Float (double-precision)") (InputAction :type "InputAction Object Reference" :default "/Game/Input/Actions/IA_Crouch.IA_Crouch"))
  (:`Started`
    (if (`NavMovementComponent.IsMovingOnGround` (`self.CharacterMovement`))
      (if (`self.Sprinting`)
        (bind _slide_started (`self.A_Slide`))
        (if _slide_started
          (`self.Crouch`)
          (bind (_direction _tlt_slidealpha) (`Timeline|TL_Slide` :!via `PlayFromStart`)
            (:`Update`
              (set `CharacterMovementComponent.MaxWalkSpeedCrouched` (`KismetMathLibrary.Lerp` 850.0 150.0 _tlt_slidealpha) (`self.CharacterMovement`)))
            (:`Finished`
              (`self.UnCrouch`)
              (set `self.Sliding` false))))
        (else
          (`self.A_Crouch`))))))

(event `EnhancedInput|/Game/Input/Actions/IA_Attack`
  (params (ActionValue :type Boolean) (ElapsedSeconds :type "Float (double-precision)") (TriggeredSeconds :type "Float (double-precision)") (InputAction :type "InputAction Object Reference" :default "/Game/Input/Actions/IA_Attack.IA_Attack"))
  (:`Triggered`
    (`KismetSystemLibrary.PrintString` "ATTACK")))

(fn `A_Crouch`
  (if (`self.Crouched`)
    (`self.UnCrouch`)
    (set `self.Crouched` false)
    (else
      (`self.Crouch`)
      (set `self.Crouched` true))))

(fn `A_Slide`
  (returns (`Slide Started` :type Boolean))
  (if (`self.Sliding`)
    (`KismetSystemLibrary.PrintString` "ALREADY SLIDING")
    (return false)
    (else
      (set `self.Sliding` true)
      (return true))))

(fn `UserConstructionScript`
  (`parent.UserConstructionScript`))